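; Door actor that swings open and closed in response to open and close requests from its OpenDoor member.
; A DoorOpen timeline plays or reverses, applying its yaw curve relative to the rotation saved at BeginPlay.
; An Audio Timing event on the timeline plays a quiet Doorlock sound at InitialLocation.
; The node that sets InitialLocation never runs, so that location is never captured from the actor.
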(event OnOpenRequest(OpenDoor)
  (bind _opendoor (Timeline|DoorOpen Play)
    (:Update
      (Transformation|SetActorRotation (Math|Rotator|CombineRotators (Math|Rotator|MakeRotator 0.0 0.0 _opendoor) (Variables|Default|GetInitialRotation))))
    (:AudioTiming
      (Audio|PlaySoundatLocation "/Game/Audio/door-lock.door-lock" (Variables|Default|GetInitialLocation) "0, 0, 0" 0.1 1.0))))

(event OnCloseRequest(OpenDoor)
  (bind _opendoor (Timeline|DoorOpen Reverse)
    (:Update
      (Transformation|SetActorRotation (Math|Rotator|CombineRotators (Math|Rotator|MakeRotator 0.0 0.0 _opendoor) (Variables|Default|GetInitialRotation))))
    (:AudioTiming
      (Audio|PlaySoundatLocation "/Game/Audio/door-lock.door-lock" (Variables|Default|GetInitialLocation) "0, 0, 0" 0.1 1.0))))

(event EventBeginPlay
  (Variables|Default|SetInitialRotation (Transformation|GetActorRotation)))

(fn ConstructionScript)